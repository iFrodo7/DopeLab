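; Sliding door that the player opens and closes with the Interactuar input, provided the first-person character holds a key (TieneLlave).
; The Box overlap enables input, shows the prompt widget and opens a Gate, then reverses all three on exit.
; With the key, a FlipFlop plays or reverses a Timeline that slides the Cube along local X.
; Without it, a locked-door sound plays and the key-required widget replaces the prompt.
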(event OnComponentBeginOverlap(Box)
  (params (OverlappedComponent :type Primitive%20Component%20Object%20Reference) (OtherActor :type Actor%20Object%20Reference) (OtherComp :type Primitive%20Component%20Object%20Reference) (OtherBodyIndex :type Integer) (bFromSweep :type Boolean) (SweepResult :type Hit%20Result%20Structure%20%28by%20ref%29))
  (bind _asfirst_person_character (Utilities|Casting|CastToFirstPersonCharacter (Game|GetPlayerCharacter 0)))
  (Input|EnableInput (Game|GetPlayerController 0))
  (Widget|SetVisibility (Variables|Default|GetWidget) "Visible")
  (Utilities|FlowControl|Gate true) ; enters at Open
)

(event OnComponentEndOverlap(Box)
  (params (OverlappedComponent :type Primitive%20Component%20Object%20Reference) (OtherActor :type Actor%20Object%20Reference) (OtherComp :type Primitive%20Component%20Object%20Reference) (OtherBodyIndex :type Integer))
  (Utilities|Casting|CastToFirstPersonCharacter (Game|GetPlayerCharacter 0))
  (Input|DisableInput (Game|GetPlayerController 0))
  (Widget|SetVisibility (Variables|Default|GetWidget) "Hidden")
  (Widget|SetVisibility (Variables|Default|GetWidget_0) "Hidden")
  (Utilities|FlowControl|Gate true) ; enters at Close
)

(event EventBeginPlay
  (bind _returnvalue (UserInterface|CreateWidget "/Game/Widgets/PuertaWidget.PuertaWidget_C"))
  (bind _returnvalue_2 (UserInterface|CreateWidget "/Game/Widgets/PuertaWidgetKey.PuertaWidgetKey_C"))
  (bind _output_get (Variables|Default|SetWidget _returnvalue))
  (bind _output_get_2 (Variables|Default|SetWidget_0 _returnvalue_2))
  (UserInterface|Viewport|AddtoViewport _output_get 0)
  (Widget|SetVisibility _output_get "Hidden"))

(event Input|ActionEvents|InputActionInteractuar
  (params (Key :type Key%20Structure))
  (:Pressed
    (if (Variables|/Game/Blueprints/FirstPersonBP/Blueprints/FirstPersonCharacter.FirstPersonCharacter_C|GetTieneLlave (stale OnComponentBeginOverlap(Box) _asfirst_person_character))
      (Utilities|FlowControl|Gate true
        (:Exit
          (Utilities|FlowControl|FlipFlop
            (:A
              (bind _newtrack_0 (Timeline|Timeline_1 Play)
                (:Update
                  (Transformation|SetRelativeLocation (Variables|Default|GetCube) (Math|Vector|MakeVector (* _newtrack_0 2e+02) 0.0 141.0) false false))))
            (:B
              (Timeline|Timeline_1 Reverse)))))
      (else
        (Audio|PlaySoundatLocation "/Game/Blueprints/Doors_Mechanic/SoundEffects/131028__dymewiz__locking-a-door-03.131028__dymewiz__locking-a-door-03" (Transformation|GetActorLocation) "0, 0, 0" 1.0 1.0 0.0 0 0 0)
        (Widget|SetVisibility (Variables|Default|GetWidget) "Hidden")
        (Widget|SetVisibility (Variables|Default|GetWidget_0) "Visible")))))

(fn ConstructionScript)

(fn InteraccionPuerta
  (params (Interactor :type Character%20Object%20Reference))
  (return false))