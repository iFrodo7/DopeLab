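; Key pickup actor for the door mechanic that lets the first-person player collect a key.
; Box overlap reveals a prompt widget, enables player input and opens a Gate; leaving hides, disables and closes them.
; Pressing Interactuar through the open gate sets TieneLlave on the character, plays a pickup sound and destroys the key.
; Overlap events cast player character 0 rather than checking the overlapping actor.
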(event OnComponentBeginOverlap(Box)
  (params (OverlappedComponent :type Primitive%20Component%20Object%20Reference) (OtherActor :type Actor%20Object%20Reference) (OtherComp :type Primitive%20Component%20Object%20Reference) (OtherBodyIndex :type Integer) (bFromSweep :type Boolean) (SweepResult :type Hit%20Result%20Structure%20%28by%20ref%29))
  (bind _asfirst_person_character (Utilities|Casting|CastToFirstPersonCharacter (Game|GetPlayerCharacter 0)))
  (Development|SetHiddeninGame (Variables|Default|GetWidget) false false)
  (Input|EnableInput (Game|GetPlayerController 0))
  (Utilities|FlowControl|Gate true) ; enters at Open
)

(event OnComponentEndOverlap(Box)
  (params (OverlappedComponent :type Primitive%20Component%20Object%20Reference) (OtherActor :type Actor%20Object%20Reference) (OtherComp :type Primitive%20Component%20Object%20Reference) (OtherBodyIndex :type Integer))
  (Utilities|Casting|CastToFirstPersonCharacter (Game|GetPlayerCharacter 0))
  (Development|SetHiddeninGame (Variables|Default|GetWidget) true false)
  (Input|DisableInput (Game|GetPlayerController 0))
  (Utilities|FlowControl|Gate true) ; enters at Close
)

(event EventBeginPlay
  (Development|SetHiddeninGame (Variables|Default|GetWidget) true false))

(event Input|ActionEvents|InputActionInteractuar
  (params (Key :type Key%20Structure :default "None"))
  (:Pressed
    (Utilities|FlowControl|Gate true
      (:Exit
        (Variables|/Game/Blueprints/FirstPersonBP/Blueprints/FirstPersonCharacter.FirstPersonCharacter_C|SetTieneLlave' (stale OnComponentBeginOverlap(Box) _asfirst_person_character) true)
        (Audio|PlaySoundatLocation "/Game/Blueprints/Doors_Mechanic/SoundEffects/267711__weejee-vdh__picking-up-keys.267711__weejee-vdh__picking-up-keys" (Transformation|GetActorLocation) "0, 0, 0" 1.0 1.0 0.0 0 0 0)
        (Actor|DestroyActor)))))

(fn ConstructionScript)