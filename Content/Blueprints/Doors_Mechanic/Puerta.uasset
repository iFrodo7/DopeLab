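; Sliding door Blueprint that toggles open and closed through an interaction call and shows an on-screen widget near it.
; InteraccionPuerta calls DoorOpening, where a FlipFlop alternately plays and reverses a timeline that slides the Cube along relative X.
; The PuertaWidget is created hidden at BeginPlay and toggled by Box overlap events.
; Those events cast player character 0 to FirstPersonCharacter without checking which actor overlapped.
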(event OnComponentBeginOverlap(Box)
  (params (OverlappedComponent :type Primitive%20Component%20Object%20Reference) (OtherActor :type Actor%20Object%20Reference) (OtherComp :type Primitive%20Component%20Object%20Reference) (OtherBodyIndex :type Integer) (bFromSweep :type Boolean) (SweepResult :type Hit%20Result%20Structure%20%28by%20ref%29))
  (Utilities|Casting|CastToFirstPersonCharacter (Game|GetPlayerCharacter 0))
  (Widget|SetVisibility (Variables|Default|GetWidget) "Visible"))

(event OnComponentEndOverlap(Box)
  (params (OverlappedComponent :type Primitive%20Component%20Object%20Reference) (OtherActor :type Actor%20Object%20Reference) (OtherComp :type Primitive%20Component%20Object%20Reference) (OtherBodyIndex :type Integer))
  (Utilities|Casting|CastToFirstPersonCharacter (Game|GetPlayerCharacter 0))
  (Widget|SetVisibility (Variables|Default|GetWidget) "Hidden"))

(event Custom|DoorOpening
  (Utilities|FlowControl|FlipFlop
    (:A
      (bind _newtrack_0 (Timeline|Timeline_0 Play)
        (:Update
          (Transformation|SetRelativeLocation (Variables|Default|GetCube) (Math|Vector|MakeVector (* _newtrack_0 2e+02) 0.0 141.0) false false))))
    (:B
      (Timeline|Timeline_0 Reverse))))

(event EventBeginPlay
  (bind _returnvalue (UserInterface|CreateWidget "/Game/Widgets/PuertaWidget.PuertaWidget_C"))
  (bind _output_get (Variables|Default|SetWidget _returnvalue))
  (UserInterface|Viewport|AddtoViewport _output_get 0)
  (Widget|SetVisibility _output_get "Hidden"))

(fn ConstructionScript)

(fn InteraccionPuerta
  (params (Interactor :type Character%20Object%20Reference))
  (CallFunction|DoorOpening)
  (return false))