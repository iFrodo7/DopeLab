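; Wardrobe hiding spot that the first-person character enters and exits with Interactuar while inside its trigger box, which also shows a prompt widget.
; Toggling hides the character, disables its collision, blends the view to the wardrobe and replays a door timeline.
; While hidden, look input drives a clamped camera through a self-calling Delay loop; otherwise it passes to the character.
; Hiding destroys the character's PawnNoiseEmitter, with no restoration here.
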(event OnComponentBeginOverlap(Box)
  (params (OverlappedComponent :type Primitive%20Component%20Object%20Reference) (OtherActor :type Actor%20Object%20Reference) (OtherComp :type Primitive%20Component%20Object%20Reference) (OtherBodyIndex :type Integer) (bFromSweep :type Boolean) (SweepResult :type Hit%20Result%20Structure%20%28by%20ref%29))
  ;[1 1 1] EntrarWardrove
  (bind _asfirst_person_character (Utilities|Casting|CastToFirstPersonCharacter OtherActor))
  (Variables|Default|SetChar%20REF _asfirst_person_character)
  (Development|SetHiddeninGame (Variables|Default|GetWidget) false false)
  (Input|EnableInput (Game|GetPlayerController 0))
  (Utilities|FlowControl|Gate true) ; enters at Open
)

(event OnComponentEndOverlap(Box)
  (params (OverlappedComponent :type Primitive%20Component%20Object%20Reference) (OtherActor :type Actor%20Object%20Reference) (OtherComp :type Primitive%20Component%20Object%20Reference) (OtherBodyIndex :type Integer))
  (bind _returnvalue (Game|GetPlayerController 0))
  ;[1 1 1] EntrarWardrove
  (Utilities|Casting|CastToFirstPersonCharacter OtherActor)
  (Development|SetHiddeninGame (Variables|Default|GetWidget) true false)
  (Input|DisableInput _returnvalue)
  (Utilities|FlowControl|Gate true) ; enters at Close
)

(event Custom|MoveCamera
  (if (Variables|Default|GetIsHiding?)
    (Transformation|SetRelativeRotation (Variables|Default|GetCamera) (Math|Rotator|MakeRotator 0.0 (* (stale Input|AxisEvents|InputAxisLookUp _output_get) -1.0) (stale Input|AxisEvents|InputAxisTurn _output_get)) false false)
    (Utilities|FlowControl|Delay 0.001)
    (CallFunction|MoveCamera)))

(event EventBeginPlay
  (Development|SetHiddeninGame (Variables|Default|GetWidget) true false))

(event Input|ActionEvents|InputActionInteractuar
  (params (Key :type Key%20Structure :default "None"))
  ;[1 1 1] EntrarWardrove
  (:Pressed
    (Utilities|FlowControl|Gate true :!label _label
      (:Exit
        (Utilities|FlowControl|Sequence
          (:then_0
            (CallFunction|ToglleHide)
            (CallFunction|MoveCamera)
            (Utilities|FlowControl|Delay 0.2)
            (Input|EnableInput (Game|GetPlayerController 0))
            (goto _label Open))
          (:then_1
            (|OpenDoor)))))))

(event Input|AxisEvents|InputAxisLookUp
  (params (AxisValue :type Float%20%28single-precision%29))
  (if (Variables|Default|GetIsHiding?)
    (bind _output_get (Variables|Default|SetPitch (Math|Float|Clamp(Float) (+ (Variables|Default|GetPitch) AxisValue) -4e+01 2e+01)))
    (else
      (Pawn|Input|AddControllerPitchInput (Variables|Default|GetChar%20REF) AxisValue))))

(event Input|AxisEvents|InputAxisTurn
  (params (AxisValue :type Float%20%28single-precision%29))
  (if (Variables|Default|GetIsHiding?)
    (bind _output_get (Variables|Default|SetYaw (Math|Float|Clamp(Float) (+ (Variables|Default|GetYaw) AxisValue) -6e+01 6e+01)))
    (else
      (Pawn|Input|AddControllerYawInput (Variables|Default|GetChar%20REF) AxisValue))))

(fn ConstructionScript)

(fn ToglleHide
  (bind _returnvalue (Game|GetPlayerController 0))
  (bind _char_ref (Variables|Default|GetChar%20REF))
  (if (Variables|Default|GetIsHiding?)
    (Variables|Default|SetIsHiding? false)
    (Rendering|SetActorHiddenInGame _char_ref false)
    (Collision|SetActorEnableCollision _char_ref true)
    (Game|Player|SetViewTargetwithBlend _returnvalue _char_ref 0.8 "VTBlend_Linear" 0.0 false)
    (else
      (Variables|Default|SetIsHiding? true)
      (Rendering|SetActorHiddenInGame _char_ref true)
      (Collision|SetActorEnableCollision _char_ref false)
      (Game|Player|SetViewTargetwithBlend _returnvalue self 0.8 "VTBlend_Linear" 0.0 false)
      (Components|DestroyComponent (Variables|/Game/Blueprints/FirstPersonBP/Blueprints/FirstPersonCharacter.FirstPersonCharacter_C|GetPawnNoiseEmitter _char_ref)))))